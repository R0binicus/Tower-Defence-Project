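; Game mode that spawns player robots at a spawn pad, both for new players and when a new robot is printed.
; It overrides new-player handling to share the spawn routine, which uses the first BP_SpawnPad found and passes it a wrapping index from the spawn counter.
; A tracked array caps the robot population by dissolving and removing the oldest when the limit is reached.
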(event `SpawnPlayerAtActiveSpawnPad`
  (bind _spawndcharacters (`self.SpawndCharacters`))
  (bind _output (`|GetArrayItem` _spawndcharacters))
  ;[0.6735 1 0.6243 1 12] The same functionality as at game start (see below) can be triggered when the player "prints" a new robot.
  ;[0.6143 1 0.5729 1 12] Spawn a new player at the active spawn pad. Give him an index between 0 and max bots. GetMaxBots is a pure library function we can call from anywhere.
  (bind _outactors (`GameplayStatics.GetAllActorsOfClass` "/Game/Blueprints/GameElements/BP_SpawnPad.BP_SpawnPad_C" :!label _label))
  (`/Game/Blueprints/GameElements/BP_SpawnPad.SpawnPlayer` (`|GetArrayItem` _outactors) (mod (`self.SpawnCounter`) 8))
  ;[0.6143 1 0.5729 1 12] if the amount of spawn characters is >= the max amount robots we allow....
  (if (>= (`KismetArrayLibrary.Array_Length` (`self.SpawndCharacters`)) 8)
    ;[1 0.8864 0.5064 1 12] ...tell the first robot in the list to dissolve itself and remove him from our array of spawned characters
    (`/Game/Blueprints/Character/BP_Bot_Import.Dissolve` _output)
    (`KismetArrayLibrary.Array_RemoveItem` _spawndcharacters _output))
  ;[0.5659 0.7811 1 1 12] ...always add the new spawned robot to the array and increase the spawn counter.
  (`KismetArrayLibrary.Array_AddUnique` (`self.SpawndCharacters`))
  (`/Engine/EditorBlueprintResources/StandardMacros.IncrementInt` (`self.SpawnCounter`)))

(event `self.HandleStartingNewPlayer`
  (params (NewPlayer :type "PlayerController Object Reference"))
  ;[0.6735 1 0.6243 1 12] This is an overwriteable function in game mode. We do not want the exsiting framework to handle it but do something own here
  (goto _label))

(fn `UserConstructionScript`)