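; Tower defence game mode meant to spawn player robots at a BP_SpawnPad, at game start or when a new robot is printed.
; HandleStartingNewPlayer is overridden to share the SpawnPlayerAtActiveSpawnPad path, which currently only gathers spawn pads.
; The disconnected remainder would spawn at the first pad with a cycling index, track robots and dissolve the oldest at the cap.
; ActiveSpawnPad is unused.
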(event `SpawnPlayerAtActiveSpawnPad`
  ;[0.6735 1 0.6243 1 12] The same functionality as at game start (see below) can be triggered when the player "prints" a new robot.
  ;[0.6143 1 0.5729 1 12] Spawn a new player at the active spawn pad. Give him an index between 0 and max bots. GetMaxBots is a pure library function we can call from anywhere.
  (bind _outactors (`GameplayStatics.GetAllActorsOfClass` "/Game/Blueprints/GameElements/BP_SpawnPad.BP_SpawnPad_C" :!label _label)))

(event `self.HandleStartingNewPlayer`
  (params (NewPlayer :type "PlayerController Object Reference"))
  ;[0.6735 1 0.6243 1 12] This is an overwriteable function in game mode. We do not want the exsiting framework to handle it but do something own here
  (goto _label))

(fn `UserConstructionScript`)