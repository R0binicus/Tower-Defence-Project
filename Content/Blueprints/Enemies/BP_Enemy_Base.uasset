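; BP_Enemy_Base is an enemy base Blueprint that adds a ragdoll-and-dissolve effect on death.
; Death calls the parent, disables capsule collision and briefly simulates mesh physics.
; It then spawns an attached dissolve effect tinted by VFXColourHue, hides the mesh, stops physics and sets a short lifespan for cleanup.
; The Dissolve function is empty, and its timer call is never run.
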(event `self.Death`
  (params (bByTurret :type Boolean))
  (`parent.Death` bByTurret)
  (`PrimitiveComponent.SetCollisionEnabled` (`self.CapsuleComponent`) "NoCollision")
  (`PrimitiveComponent.SetCollisionEnabled` (`self.Mesh`) "QueryAndPhysics")
  (`SkeletalMeshComponent.SetAllBodiesBelowSimulatePhysics` (`self.Mesh`) "head" true true)
  (`PrimitiveComponent.SetSimulatePhysics` (`self.Mesh`) true)
  (`KismetSystemLibrary.Delay` 0.1)
  (bind _returnvalue (`NiagaraFunctionLibrary.SpawnSystemAttached` "/Game/FX/Dissolve/FX_CharacterDissolve.FX_CharacterDissolve" (`self.Mesh`) "None" (0.0 0.0 0.0) (struct) "KeepRelativeOffset" true))
  (`FXSystemComponent.SetColorParameter` _returnvalue "AntBotColor" (make `LinearColor` (`self.VFXColourHue`) 0.0 0.0 1.0))
  (`SceneComponent.SetVisibility` (`self.Mesh`) false false)
  (`KismetSystemLibrary.Delay` 0.1)
  (`PrimitiveComponent.SetSimulatePhysics` (`self.Mesh`) false)
  (`PrimitiveComponent.SetCollisionEnabled` (`self.Mesh`) "NoCollision")
  (`self.SetLifeSpan` 4.0))

(fn `Dissolve`)

(fn `UserConstructionScript`)